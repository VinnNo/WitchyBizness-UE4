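; Breakable block that crumbles shortly after the witch character touches it.
; On begin play the sprite flipbook is stopped on its first frame with looping off.
; An overlap of OverlapBox by cWitch plays the animation after a short delay, disables Box collision partway through, and destroys the actor when playback finishes.
; The Box hit handler tests for a vertical normal but performs no action.
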(event `self.ReceiveBeginPlay`
  (`PaperFlipbookComponent.SetLooping` (`self.Sprite`) false)
  (`PaperFlipbookComponent.Stop` (`self.Sprite`))
  (`PaperFlipbookComponent.SetPlaybackPosition` (`self.Sprite`) 0.0 false))

(event `self.Box.OnComponentHit`
  (params (HitComponent :type "PrimitiveComponent Object Reference") (OtherActor :type "Actor Object Reference") (OtherComp :type "PrimitiveComponent Object Reference") (NormalImpulse :type "Vector Structure") (Hit :type "HitResult Structure (by ref)"))
  (cast `cWitch` OtherActor)
  (if (== (.z (`.Normal` (`GameplayStatics.BreakHitResult` Hit))) -1.0)
    _))

(event `self.OverlapBox.OnComponentBeginOverlap`
  (params (OverlappedComponent :type "PrimitiveComponent Object Reference") (OtherActor :type "Actor Object Reference") (OtherComp :type "PrimitiveComponent Object Reference") (OtherBodyIndex :type Integer) (bFromSweep :type Boolean) (SweepResult :type "HitResult Structure (by ref)"))
  (cast `cWitch` OtherActor)
  (`KismetSystemLibrary.Delay` 0.2)
  (`PaperFlipbookComponent.PlayFromStart` (`self.Sprite`))
  (`KismetSystemLibrary.Delay` 0.15)
  (`PrimitiveComponent.SetCollisionEnabled` (`self.Box`) "NoCollision"))

(event `self.Sprite.OnFinishedPlaying`
  (`self.K2_DestroyActor`))

(fn `UserConstructionScript`)