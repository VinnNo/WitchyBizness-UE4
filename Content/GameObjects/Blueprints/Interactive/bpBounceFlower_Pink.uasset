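; Pink bounce flower interactive that springs the player's witch character into the air.
; DoOverlap launches the bpWitch player vertically at LaunchStrength, overriding existing velocity, refills its LaunchCount to the maximum and plays the flower's sprite animation.
; The sprite is held stopped on its first frame at BeginPlay and resets there whenever playback finishes.
; DoOverlap has no caller in this graph; the local overlap event is disabled.
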(event `self.ReceiveBeginPlay`
  (`PaperFlipbookComponent.SetLooping` (`self.Sprite`) false :!label _label)
  (`PaperFlipbookComponent.Stop` (`self.Sprite`))
  (`PaperFlipbookComponent.SetPlaybackPositionInFrames` (`self.Sprite`) 0 false)
  (set `self.TargetActor` (`GameplayStatics.GetPlayerCharacter` 0)))

(event `ResetSprite`
  (goto _label))

(event `self.DoOverlap`
  (bind _asbp_witch (cast `/Game/GameObjects/Blueprints/Player/bpWitch` (`GameplayStatics.GetPlayerCharacter` 0)))
  (`Character.LaunchCharacter` _asbp_witch (`KismetMathLibrary.MakeVector` 0.0 0.0 (`self.LaunchStrength`)) true true)
  (set `cWitch.LaunchCount` (`cWitch.LaunchCountMax` _asbp_witch) _asbp_witch)
  (`PaperFlipbookComponent.PlayFromStart` (`self.Sprite`)))

(event `self.Sprite.OnFinishedPlaying`
  (`self.ResetSprite`))

(fn `UserConstructionScript`)