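; Health pickup that homes in on the bpWitch player, granting hitpoints and money on contact.
; At BeginPlay its detection sphere copies the witch's pickup radius; overlapping it starts a self-repeating short-delay loop that re-aims projectile movement, slow at first, then much faster.
; Sprite overlap applies scaled healing, adds money (multiplier scales the existing total), then spawns a disperse actor and destroys the pickup.
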(event `self.ReceiveBeginPlay`
  (bind _asbp_witch (cast `/Game/GameObjects/Blueprints/Player/bpWitch` (`GameplayStatics.GetPlayerCharacter` 0)))
  (`SphereComponent.SetSphereRadius` (`self.Sphere`) (`SphereComponent.GetScaledSphereRadius` (`/Game/GameObjects/Blueprints/Player/bpWitch.PickupCollision` _asbp_witch)) true))

(event `self.PaperSprite.OnComponentBeginOverlap`
  (params (OverlappedComponent :type "PrimitiveComponent Object Reference") (OtherActor :type "Actor Object Reference") (OtherComp :type "PrimitiveComponent Object Reference") (OtherBodyIndex :type Integer) (bFromSweep :type Boolean) (SweepResult :type "HitResult Structure (by ref)"))
  (bind _asbp_witch (cast `/Game/GameObjects/Blueprints/Player/bpWitch` OtherActor))
  (`cWitch.DoSetHitpoints` _asbp_witch (* (`self.Value`) (`cWitch.PickupHealingMultiplier` _asbp_witch)))
  (set `cWitch.MoneyCount` (+ (`self.MoneyValue`) (* (`cWitch.MoneyCount` _asbp_witch) (`cWitch.PickupMoneyMultiplier` _asbp_witch))) _asbp_witch)
  (`self.DestroyingEvent`))

(event `DestroyingEvent`
  (`|SpawnActorFromClass` "/Game/GameObjects/Blueprints/Pickups/bpHpDisperse.bpHpDisperse_C" (`self.GetTransform`) "Undefined" "OverrideRootScale" null null)
  (`self.K2_DestroyActor`))

(event `self.Sphere.OnComponentBeginOverlap`
  (params (OverlappedComponent :type "PrimitiveComponent Object Reference") (OtherActor :type "Actor Object Reference") (OtherComp :type "PrimitiveComponent Object Reference") (OtherBodyIndex :type Integer) (bFromSweep :type Boolean) (SweepResult :type "HitResult Structure (by ref)"))
  (if (== (`self.bIsSeeking`) false)
    (`self.TurnOnSeeking` OtherActor)))

(event `TurnOnSeeking`
  (params (OtherActor :type "Actor Object Reference"))
  (bind _projectilemovement (`self.ProjectileMovement`))
  (bind _asbp_witch (cast `/Game/GameObjects/Blueprints/Player/bpWitch` OtherActor))
  (`|ExecutionSequence`
    (:`then_0`
      (bind _tossvelocity (`GameplayStatics.BlueprintSuggestProjectileVelocity` (`self.K2_GetActorLocation`) (`self.K2_GetActorLocation` _asbp_witch) 500.0 0.0 "DoNotTrace"))
      (set `MovementComponent.Velocity` _tossvelocity _projectilemovement)
      (`ActorComponent.Activate` _projectilemovement false)
      (`KismetSystemLibrary.Delay` 0.0016)
      (`/Engine/EditorBlueprintResources/StandardMacros.IsValid` self
        (:`Is Valid`
          (`self.TurnOnSeeking` _asbp_witch))))
    (:`then_1`
      (if (`self.bIsSeeking`)
        (if (< (`ProjectileMovementComponent.MaxSpeed` (`self.ProjectileMovement`)) 800.0)
          (`KismetSystemLibrary.Delay` 0.5)
          (set `ProjectileMovementComponent.MaxSpeed` 2000.0 (`self.ProjectileMovement`)))
        (else
          (set `self.bIsSeeking` true)
          (set `ProjectileMovementComponent.MaxSpeed` 100.0 (`self.ProjectileMovement`)))))))

(fn `UserConstructionScript`)