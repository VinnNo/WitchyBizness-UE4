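; Plasma Demon enemy Blueprint that deals contact damage to the witch player and can be hit by player shots.
; Capsule overlaps apply contact damage, pass shot damage into GetHit, or set the turn flag on meeting another enemy.
; DeathSequenceEvent spawns a death actor at the particle location, and the actor destroys itself when the sprite flipbook finishes playing in state 14.
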(event `self.CapsuleComponent.OnComponentBeginOverlap`
  (params (OverlappedComponent :type "PrimitiveComponent Object Reference") (OtherActor :type "Actor Object Reference") (OtherComp :type "PrimitiveComponent Object Reference") (OtherBodyIndex :type Integer) (bFromSweep :type Boolean) (SweepResult :type "HitResult Structure (by ref)"))
  ;[1 0 0] Collision
  ;;[1 0.103 0.0831] Hit Player
  (bind _asbp_witch (cast `/Game/GameObjects/Blueprints/Player/bpWitch` OtherActor)
    (:`then`
      (`cWitch.DoGetHit` _asbp_witch (`self.contactDamageCurrent`) (`self.K2_GetActorLocation`)))
    (:`CastFailed`
      ;;[1 0.05673 0.7923] Get hit by Shots
      (bind _asc_player_shot (cast `cPlayerShot` OtherActor)
        (:`then`
          (`/Engine/EditorBlueprintResources/StandardMacros.IsValid` _asc_player_shot
            (:`Is Valid`
              (`self.GetHit` (`cPlayerShot.attDamage` _asc_player_shot)))))
        (:`CastFailed`
          ;;[0 1 0.07465] Other Enemies
          (bind _asc_enemy_parent (cast `cEnemyParent` OtherActor))
          (set `self.bShouldDoTurn` (!= _asc_enemy_parent self)))))))

(event `self.Sprite.OnFinishedPlaying`
  ;[0 1 0.005877 0.5] Death Event
  (if (== (`self.STATE`) 14)
    (`self.K2_DestroyActor`)))

(event `self.DeathSequenceEvent`
  ;[0 1 0.005877 0.5] Death Event
  (`|SpawnActorFromClass` "/Game/GameObjects/Blueprints/Enemies/bpEnemyDeath.bpEnemyDeath_C" (`SceneComponent.K2_GetComponentToWorld` (`self.ParticleLoc`)) "Undefined" "OverrideRootScale" null null))

(fn `UserConstructionScript`)