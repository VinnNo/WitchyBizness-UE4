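; Player witch Blueprint that handles the spawning and effects side of charged shooting and double jumping.
; MakeShotEvent spawns a small, medium or large shot at ShotPosComp based on ChargeState, nudged along Y.
; Charge and release events toggle two particle systems, and double jumps spawn a dust emitter.
; It also handles pause toggling, quitting via Escape or Android Back, and debug prints, while CheckForWalls is an empty stub.
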(event `InputAxis|kDebug`
  (params (AxisValue :type "Float (single-precision)"))
  ;[1 0 0.09604] Debug Stuff
  (if (> AxisValue 0.0)
    (`self.CheckForWalls`)
    (`KismetSystemLibrary.Delay` 0.05)
    (`KismetSystemLibrary.PrintString` (`KismetStringLibrary.Conv_VectorToString` (`self.GetVelocity`)))))

(event `Key|Escape`
  (params (Key :type "Key Structure"))
  ;[1 0 0.09604] Debug Stuff
  (:`Pressed`
    (`KismetSystemLibrary.QuitGame` null "Quit" :!label _label)))

(event `Key|Android_Back`
  (params (Key :type "Key Structure"))
  ;[1 0 0.09604] Debug Stuff
  (:`Pressed`
    (goto _label)))

(event `self.MakeShotEvent`
  (bind _returnvalue (`SceneComponent.K2_GetComponentToWorld` (`self.ShotPosComp`)))
  (bind _returnvalue_2 (`KismetMathLibrary.MakeTransform` (`KismetMathLibrary.MakeVector` (.x (.location _returnvalue)) (+ (.y (.location _returnvalue)) 1.0) (.z (.location _returnvalue))) (.rotation _returnvalue) (.scale _returnvalue)))
  ;[0.9815 0.1329 1] Shoot
  (switch `int` (`self.ChargeState`)
    (:`0`
      (`|SpawnActorFromClass` "/Game/GameObjects/Blueprints/Player/bpPlayerShot_Small.bpPlayerShot_Small_C" _returnvalue_2 "Undefined" "OverrideRootScale" null null))
    (:`1`
      (`|SpawnActorFromClass` "/Game/GameObjects/Blueprints/Player/bpPlayerShot_Medium.bpPlayerShot_Medium_C" _returnvalue_2 "Undefined" "OverrideRootScale" null null))
    (:`2`
      (`|SpawnActorFromClass` "/Game/GameObjects/Blueprints/Player/bpPlayerShot_Large.bpPlayerShot_Large_C" _returnvalue_2 "Undefined" "OverrideRootScale" null null))))

(event `self.OnDoubleJumped`
  (bind (_returnvalue_location _returnvalue_rotation _returnvalue_scale) (`KismetMathLibrary.BreakTransform` (`self.GetTransform`)))
  (`GameplayStatics.SpawnEmitterAtLocation` "/Game/Particles/Particles/pDoubleJumpDust.pDoubleJumpDust" _returnvalue_location _returnvalue_rotation _returnvalue_scale))

(event `self.IsChargingEvent`
  ;[1 0.3957 0.9408] Charging
  (`ActorComponent.Activate` (`self.IsChargedParticleSystem`) false))

(event `self.IsChargedEvent`
  ;[1 0.3957 0.9408] Charging
  (`ActorComponent.Activate` (`self.ChargingParticleSystem`) false)
  (`ActorComponent.Activate` (`self.IsChargedParticleSystem`) false))

(event `InputAction|kPause` :consume false :paused true
  (params (Key :type "Key Structure"))
  (:`Released`
    (if (`GameplayStatics.IsGamePaused`)
      (`GameplayStatics.SetGamePaused` false)
      (else
        (`GameplayStatics.SetGamePaused` true)))))

(event `self.ShotReleasedEvent`
  ;[1 0.3957 0.9408] Charging
  (`ActorComponent.Deactivate` (`self.IsChargedParticleSystem`))
  (`ActorComponent.Deactivate` (`self.ChargingParticleSystem`)))

(event `CheckForWalls`)

(event `self.CapsuleComponent.OnInputTouchBegin`
  (params (FingerIndex :type "ETouchIndex Enum" :default "Touch1") (TouchedComponent :type "PrimitiveComponent Object Reference"))
  (`KismetSystemLibrary.PrintString` "Hello"))

(fn `UserConstructionScript`)