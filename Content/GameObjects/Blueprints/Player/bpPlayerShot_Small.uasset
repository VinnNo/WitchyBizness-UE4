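; Small projectile fired by the player witch, which returns one shot to her when it is destroyed.
; On BeginPlay it copies the attack damage from the player's bpWitch.
; A collision hit or overlap starts a configurable delay before destruction, while OnDeath destroys it immediately.
; Both paths run DestroyingEvent, which calls DoRegenShots on the witch before destroying the actor.
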(event `self.ReceiveBeginPlay`
  (if (`KismetSystemLibrary.IsValid` self)
    (bind _asbp_witch (cast `/Game/GameObjects/Blueprints/Player/bpWitch` (`GameplayStatics.GetPlayerCharacter` 0)))
    (set `self.attDamage` (`cWitch.attDamage` _asbp_witch))))

(event `DestroyingEvent`
  (bind _asbp_witch (cast `/Game/GameObjects/Blueprints/Player/bpWitch` (`GameplayStatics.GetPlayerCharacter` 0))
    (:`then`
      (`cWitch.DoRegenShots` _asbp_witch 1))
    (:`CastFailed`
      _))
  (`self.K2_DestroyActor`))

(event `self.OnDeath`
  (`self.DestroyingEvent` :!label _label))

(event `self.CollisionComp.OnComponentHit`
  (params (HitComponent :type "PrimitiveComponent Object Reference") (OtherActor :type "Actor Object Reference") (OtherComp :type "PrimitiveComponent Object Reference") (NormalImpulse :type "Vector Structure") (Hit :type "HitResult Structure (by ref)"))
  (`KismetSystemLibrary.Delay` (`self.DestroyDelay`) :!label _label_2)
  (goto _label))

(event `self.CollisionComp.OnComponentBeginOverlap`
  (params (OverlappedComponent :type "PrimitiveComponent Object Reference") (OtherActor :type "Actor Object Reference") (OtherComp :type "PrimitiveComponent Object Reference") (OtherBodyIndex :type Integer) (bFromSweep :type Boolean) (SweepResult :type "HitResult Structure (by ref)"))
  (goto _label_2))

(fn `UserConstructionScript`)