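; HUD manager actor that puts the in-game HUD on screen when play begins.
; BeginPlay calls the GetGameplayHud event, which creates a BpInGameHud widget, stores it and adds it to the viewport.
; Disconnected leftover nodes would clear all widgets first or create on-screen buttons when bpWitch reports a touch screen, but neither path runs.
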(event `self.ReceiveBeginPlay`
  (`self.GetGameplayHud`))

(event `GetGameplayHud`
  (`|ExecutionSequence`
    (:`then_0`
      (bind _returnvalue (`|CreateWidget` "/Game/GameObjects/Blueprints/GameManagement/bpInGameHud.bpInGameHud_C"))
      (set `self.InGameHud` _returnvalue)
      (`UserWidget.AddToViewport` (`self.InGameHud`) 0))))

(fn `UserConstructionScript`)